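; BP_SortGameMode is a game mode Blueprint that drives a sorting demo through the SortInstance game instance.
; On BeginPlay it casts to that instance, then repeatedly sets a random Height on it and calls SpawnSortingObject.
; Tick accumulates time and, past five seconds, calls Sort and prints a debug string every frame, as the timer never resets.
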(event EventBeginPlay
  (bind _assort_instance (Utilities|Casting|CastToSortInstance (Game|GetGameInstance)))
  (for _index (range 0 10)
    (Variables|/Script/GIMATTest.SortInstance|SetHeight _assort_instance (* (+ (Math|Random|RandomFloat) 1.0) 5.0))
    (Class|SortInstance|SpawnSortingObject _assort_instance)))

(event EventTick
  (params (DeltaSeconds :type Float%20%28single-precision%29))
  (bind _output_get (Variables|Default|SetTime (+ DeltaSeconds (Variables|Default|GetTime))))
  (if (> _output_get 5.0)
    (Class|SortInstance|Sort (stale EventBeginPlay _assort_instance) 0.0)
    (Development|PrintString "Hello")))

(fn ConstructionScript)